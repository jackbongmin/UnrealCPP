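; BP_ActionPlayer is a player Blueprint that keeps a state bar widget showing its health and stamina.
; Every Tick, it casts the user object of its Widget component to WB_StateBar and stops if the cast fails.
; It then sets the bar's stamina and health percentages from the current-to-max ratios held in Resource.
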(event EventTick
  (params (DeltaSeconds :type Float%20%28single-precision%29))
  (bind _resource (Variables|Default|GetResource))
  (bind _aswb_state_bar (Utilities|Casting|CastToWB_StateBar (UserInterface|GetUserWidgetObject (Variables|Default|GetWidget))))
  (Default|SetProgressPercentStamina _aswb_state_bar (/ (Variables|/Script/UnrealCpp.ResourceComponent|GetCurrentStamina _resource) (Variables|/Script/UnrealCpp.ResourceComponent|GetMaxStamina _resource)))
  (Default|SetProgressPercentHealth _aswb_state_bar (/ (Variables|/Script/UnrealCpp.ResourceComponent|GetCurrentHealth _resource) (Variables|/Script/UnrealCpp.ResourceComponent|GetMaxHealth _resource))))

(fn ConstructionScript)